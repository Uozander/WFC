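; BP_Shape3 procedurally builds a randomly tall, tapering stack of static mesh segments from its construction script.
; Each floor's random pick from the current Type's mesh array also sets the next Type, chaining segments like a simple state machine.
; Footprint scale shrinks as Base0 drops per floor, except two transition meshes that get a fixed scale.
; The Upside flip value is computed but never applied.
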(event Custom|CE_Begin
  (Variables|Default|SetInstance 1)
  (bind _output_get (Variables|Default|SetHeight (Math|Random|RandomInteger 100)))
  (Utilities|Array|SetArrayElem (Variables|Default|GetEmpty) _output_get false true)
  (for (_ _array_index) (Variables|Default|GetEmpty)
    (if (>= (Variables|Default|GetBase_0) 0.0)
      (CallFunction|CEBuild (Math|Conversions|ToFloat(Integer) _array_index))
      (Variables|Default|SetBase_0 (- (Variables|Default|GetBase_0) 0.5)))))

(event Custom|CE_Build
  (params (Floor :type Float%20%28double-precision%29))
  (Variables|Default|SetFloor Floor)
  (switch int (Variables|Default|GetType)
    (:0
      (bind _random (Utilities|Entropy (Variables|Default|GetMesh_THREE)))
      (if (== _random 0)
        (Variables|Default|SetUpside 1.8e+02)
        (else
          (Variables|Default|SetUpside 0.0)))
      (CallFunction|CEFloor (Variables|Default|GetFloor) (Variables|Default|GetSelection))
      (Variables|Default|SetType (Variables|Default|GetRandom)))
    (:1
      (bind _random_2 (Utilities|Entropy (Variables|Default|GetMesh_FOUR)))
      (switch int _random_2
        (:0
          (Variables|Default|SetUpside (+ (Variables|Default|GetUpside) 1.8e+02) :!label _label))
        (:1
          (goto _label))
        (:2
          _)
        (:3
          (Variables|Default|SetUpside (+ (Variables|Default|GetUpside) 1.8e+02))))
      (CallFunction|CEFloor (Variables|Default|GetFloor) (Variables|Default|GetSelection))
      (Variables|Default|SetType (Variables|Default|GetRandom)))
    (:2
      (Variables|Default|SetUpside 0.0)
      (Utilities|Entropy (Variables|Default|GetMesh_FIVE))
      (CallFunction|CEFloor (Variables|Default|GetFloor) (Variables|Default|GetSelection))
      (Variables|Default|SetType (Variables|Default|GetRandom)))
    (:3
      (Variables|Default|SetUpside 0.0)
      (bind _random_3 (Utilities|Entropy (Variables|Default|GetMesh_SIX)))
      (switch int _random_3
        (:0
          (Variables|Default|SetUpside (+ (Variables|Default|GetUpside) 1.8e+02) :!label _label_2))
        (:1
          (goto _label_2))
        (:2
          (Variables|Default|SetUpside (+ (Variables|Default|GetUpside) 1.8e+02))))
      (CallFunction|CEFloor (Variables|Default|GetFloor) (Variables|Default|GetSelection))
      (Variables|Default|SetType (+ (Variables|Default|GetRandom) 1)))))

(event Custom|CE_Floor
  (params (Floor :type Float%20%28double-precision%29) (Object :type Static%20Mesh%20Object%20Reference))
  (if (or (== Object "/Game/Shapes/CIRC_SM_to_MED.CIRC_SM_to_MED") (== Object "/Game/Shapes/SM_to_MED.SM_to_MED"))
    (Variables|Default|SetAwkward (/ (Variables|Default|GetBase_0) 5.0)))
  (Variables|Default|SetScale (/ (/ (Variables|Default|GetBase_0) (Variables|Default|GetAwkward)) 2.0))
  (bind _returnvalue (AddComponent|AddStaticMeshComponent false (Math|Transform|MakeTransform (Math|Vector|MakeVector 0.0 0.0 (* Floor 1e+02)) (Math|Rotator|MakeRotator 0.0 0.0 0.0) (Math|Vector|MakeVector (Variables|Default|GetScale) (Variables|Default|GetScale) 12.0))))
  (Variables|Default|SetAwkward 1.0)
  (Components|StaticMesh|SetStaticMesh _returnvalue Object))

(event EventBeginPlay
  (bind _base (Variables|Default|GetBase))
  (Variables|Default|SetBase_0 _base)
  (Variables|Default|SetScale _base))

(fn ConstructionScript
  (CallFunction|CEBegin))