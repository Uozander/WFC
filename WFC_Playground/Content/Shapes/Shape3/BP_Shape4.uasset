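; BP_Shape4 procedurally builds a tapering tower of stacked static mesh floors on BeginPlay, with a random floor count.
; Each floor picks a random shape from MeshALL via Entropy, spawns it as a component and shrinks the base scale.
; When the shape type changes, CE_Transition selects a mesh from per-type arrays and raises a shared height offset.
; The type 3 transition branch selects a mesh but never spawns it.
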(event Custom|CE_Begin
  (Variables|Default|SetOffset 0.0)
  (Variables|Default|SetInstance 1)
  (bind _output_get (Variables|Default|SetHeight (+ (Math|Random|RandomInteger (Variables|Default|GetMax%20Floors)) 5)))
  (Utilities|Array|SetArrayElem (Variables|Default|GetEmpty) _output_get false true)
  (for (_ _array_index) (Variables|Default|GetEmpty)
    (if (>= (Variables|Default|GetBase_0) 0.0)
      (Variables|Default|SetFloor (Math|Conversions|ToFloat(Integer) _array_index))
      (CallFunction|CEBuild (Math|Conversions|ToFloat(Integer) _array_index))
      (Variables|Default|SetBase_0 (- (Variables|Default|GetBase_0) (/ (Variables|Default|GetBase_0) (Variables|Default|GetHeight)))))))

(event Custom|CE_Build
  (params (Floor :type Float%20%28double-precision%29))
  (bind _mesh_all (Variables|Default|GetMesh_ALL))
  (Variables|Default|SetFloor Floor)
  (switch int (Variables|Default|GetType)
    (:0
      (bind _random (Utilities|Entropy _mesh_all))
      (if (== _random (Variables|Default|GetType))
        _
        (else
          (CallFunction|CETransition))))
    (:1
      (bind _random_2 (Utilities|Entropy _mesh_all))
      (if (== _random_2 (Variables|Default|GetType))
        _
        (else
          (CallFunction|CETransition))))
    (:2
      (bind _random_3 (Utilities|Entropy _mesh_all))
      (if (== _random_3 (Variables|Default|GetType))
        _
        (else
          (CallFunction|CETransition))))
    (:3
      (bind _random_4 (Utilities|Entropy _mesh_all))
      (if (== _random_4 (Variables|Default|GetType))
        _
        (else
          (CallFunction|CETransition)))))
  (CallFunction|CEFloorgen))

(event Custom|CE_Floor
  (params (Floor :type Float%20%28double-precision%29) (Object :type Static%20Mesh%20Object%20Reference))
  (bind _multiply (Variables|Default|GetMultiply))
  (bind _base_0 (Variables|Default|GetBase_0))
  (bind _floorheight (Variables|Default|GetFloorHeight))
  (bind _returnvalue (* _base_0 _multiply))
  (Development|PrintString (Utilities|String|ToString(Float) Floor) true true "(R=1.000000,G=0.000000,B=0.777914,A=1.000000)" 2e+01)
  (bind _returnvalue_2 (AddComponent|AddStaticMeshComponent false (Math|Transform|MakeTransform (Math|Vector|MakeVector 0.0 0.0 (+ (* Floor (* _floorheight 24.01)) (* (Variables|Default|GetOffset) 24.01))) (Math|Rotator|MakeRotator 0.0 0.0 0.0) (Math|Vector|MakeVector _returnvalue _returnvalue _floorheight))))
  (Components|StaticMesh|SetStaticMesh _returnvalue_2 Object))

(event Custom|CE_Floorgen
  (CallFunction|CEFloor (Variables|Default|GetFloor) (Variables|Default|GetSelection))
  (Variables|Default|SetType (Variables|Default|GetRandom)))

(event Custom|CE_Transition
  (bind _base_0 (Variables|Default|GetBase_0))
  (bind _floorheight (Variables|Default|GetFloorHeight))
  (bind _multiply (Variables|Default|GetMultiply))
  (bind _returnvalue (* _base_0 _multiply))
  (Variables|Default|SetFloor 0.0)
  (Variables|Default|SetOffset (+ (Variables|Default|GetOffset) 0.5))
  (switch int (Variables|Default|GetType)
    (:0
      (Variables|Default|SetTransition (Utilities|Array|Get(acopy) (Variables|Default|GetMesh_THREE) (- (Variables|Default|GetRandom) 1)))
      (bind _returnvalue_2 (AddComponent|AddStaticMeshComponent false (Math|Transform|MakeTransform (Math|Vector|MakeVector 0.0 0.0 (+ (* (Variables|Default|GetFloor) (* _floorheight 24.01)) (* (Variables|Default|GetOffset) 24.01))) (Math|Rotator|MakeRotator 0.0 0.0 0.0) (Math|Vector|MakeVector _returnvalue _returnvalue _floorheight)) :!label _label))
      (Components|StaticMesh|SetStaticMesh _returnvalue_2 (Variables|Default|GetTransition)))
    (:1
      (if (> (Variables|Default|GetRandom) 1)
        (Variables|Default|SetTransition (Utilities|Array|Get(acopy) (Variables|Default|GetMesh_FOUR) (- (Variables|Default|GetRandom) 1)))
        (goto _label)
        (else
          (Variables|Default|SetTransition (Utilities|Array|Get(acopy) (Variables|Default|GetMesh_FOUR) (Variables|Default|GetRandom)))
          (goto _label))))
    (:2
      (if (== (Variables|Default|GetRandom) 3)
        (Variables|Default|SetTransition (Utilities|Array|Get(acopy) (Variables|Default|GetMesh_FIVE) 2))
        (goto _label)
        (else
          (Variables|Default|SetTransition (Utilities|Array|Get(acopy) (Variables|Default|GetMesh_FIVE) (Variables|Default|GetRandom)))
          (goto _label))))
    (:3
      (Variables|Default|SetTransition (Utilities|Array|Get(acopy) (Variables|Default|GetMesh_SIX) (Variables|Default|GetRandom))))))

(event EventBeginPlay
  (Variables|Default|SetBase_0 (Variables|Default|GetBase))
  (CallFunction|CEBegin))

(event EventTick
  (params (DeltaSeconds :type Float%20%28single-precision%29)))

(fn ConstructionScript)