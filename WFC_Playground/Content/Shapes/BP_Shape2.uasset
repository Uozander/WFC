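; BP_Shape2 procedurally stacks random static meshes into a tower-like shape from the Construction Script.
; CE_Begin rolls a floor count, calling CE_Build while Base, which shrinks each floor, stays non-negative.
; CE_Build picks a mesh from the array chosen by Type; CE_Floor places it with random yaw and Base-scaled random width, except CIRC_SM_to_MED, which cancels Base.
; Logic randomizing Type and Upside is disconnected.
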(event Custom|CE_Begin
  (Variables|Default|SetInstance 1)
  (bind _output_get (Variables|Default|SetHeight (Math|Random|RandomInteger 100)))
  (Utilities|Array|SetArrayElem (Variables|Default|GetEmpty) _output_get false true)
  (for (_ _array_index) (Variables|Default|GetEmpty)
    (if (>= (Variables|Default|GetBase) 0.0)
      (CallFunction|CEBuild (Math|Conversions|ToFloat(Integer) _array_index))
      (Variables|Default|SetBase (- (Variables|Default|GetBase) 0.5)))))

(event Custom|CE_Build
  (params (Floor :type Float%20%28double-precision%29))
  (bind _mesh_circ (Variables|Default|GetMesh_CIRC))
  (bind _mesh_circ_sm_to_med (Variables|Default|GetMesh_Circ_SM_to_MED))
  (bind _mesh_basic (Variables|Default|GetMesh_Basic))
  (bind _mesh_sm_to_med (Variables|Default|GetMesh_SM_to_MED))
  (switch int (Variables|Default|GetType)
    (:0
      (CallFunction|CEFloor Floor (Utilities|Array|Get(acopy) _mesh_circ (Math|Random|RandomInteger (Utilities|Array|Length _mesh_circ)))))
    (:1
      (CallFunction|CEFloor Floor (Utilities|Array|Get(acopy) _mesh_circ_sm_to_med (Math|Random|RandomInteger (Utilities|Array|Length _mesh_circ_sm_to_med)))))
    (:2
      (CallFunction|CEFloor Floor (Utilities|Array|Get(acopy) _mesh_basic (Math|Random|RandomInteger (Utilities|Array|Length _mesh_basic)))))
    (:3
      (CallFunction|CEFloor Floor (Utilities|Array|Get(acopy) _mesh_sm_to_med (Math|Random|RandomInteger (Utilities|Array|Length _mesh_sm_to_med)))))))

(event Custom|CE_Floor
  (params (Floor :type Float%20%28double-precision%29) (Object :type Static%20Mesh%20Object%20Reference))
  (if (== Object "/Game/Shapes/CIRC_SM_to_MED.CIRC_SM_to_MED")
    (Variables|Default|SetAwkward (Variables|Default|GetBase)))
  (bind _returnvalue (AddComponent|AddStaticMeshComponent false (Math|Transform|MakeTransform (Math|Vector|MakeVector 0.0 0.0 (* Floor 1e+02)) (Math|Rotator|MakeRotator (Variables|Default|GetUpside) 0.0 (* (Math|Random|RandomFloat) 3.6e+02)) (Math|Vector|MakeVector (+ (/ (* (Math|Random|RandomFloat) (Variables|Default|GetBase)) (Variables|Default|GetAwkward)) 0.5) (+ (/ (* (Math|Random|RandomFloat) (Variables|Default|GetBase)) (Variables|Default|GetAwkward)) 0.5) 1.0))))
  (Variables|Default|SetAwkward 1.0)
  (Components|StaticMesh|SetStaticMesh _returnvalue Object))

(fn ConstructionScript
  (CallFunction|CEBegin))