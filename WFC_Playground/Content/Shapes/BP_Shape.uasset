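; BP_Shape is an actor that procedurally stacks random meshes into a vertical column at BeginPlay.
; It randomizes the base mesh, then resizes a bool array to a random height as a loop counter for the build event.
; Each piece copies the previous component's transform at a fixed Z spacing, with mesh type 1 pitched upside down.
; Building continues only while Type is 0, so any other random type ends the stack.
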(event Custom|CE_BEGIN
  (bind _new_mesh (Variables|Default|GetNew%20Mesh))
  (Components|StaticMesh|SetStaticMesh (Variables|Default|GetStaticMesh) (Utilities|Array|Get(acopy) _new_mesh (Math|Random|RandomInteger (Utilities|Array|Length _new_mesh))))
  (Variables|Default|SetHeight (* (Math|Random|RandomFloat) 1e+02))
  (Utilities|Array|SetArrayElem (Variables|Default|GetEmpty) (Math|Float|Truncate (Variables|Default|GetHeight)) true true)
  (for (_ _array_index) (Variables|Default|GetEmpty)
    (CallFunction|CEBUILD (Math|Conversions|ToFloat(Integer) _array_index))))

(event Custom|CE_BUILD
  (params (Index :type Float%20%28double-precision%29))
  (switch int (Variables|Default|GetType)
    (:0
      (bind _output_get (Variables|Default|SetType (Math|Random|RandomInteger (Utilities|Array|Length (Variables|Default|GetNew%20Mesh)))))
      (if (== _output_get 1)
        (Variables|Default|SetUpside 1.8e+02)
        (else
          (Variables|Default|SetUpside 0.0)))
      (bind _returnvalue (AddComponent|AddStaticMeshComponent false (Math|Transform|MakeTransform (Math|Vector|MakeVector (.x (.location (Transformation|GetRelativeTransform (Variables|Default|GetShape)))) (.y (.location (Transformation|GetRelativeTransform (Variables|Default|GetShape)))) (* 1e+02 Index)) (Math|Rotator|MakeRotator (.Roll (Math|Rotator|BreakRotator (.rotation (Transformation|GetRelativeTransform (Variables|Default|GetShape))))) (+ (.Pitch (Math|Rotator|BreakRotator (.rotation (Transformation|GetRelativeTransform (Variables|Default|GetShape))))) (Variables|Default|GetUpside)) (.Yaw (Math|Rotator|BreakRotator (.rotation (Transformation|GetRelativeTransform (Variables|Default|GetShape)))))) (Math|Vector|MakeVector (.x (.scale (Transformation|GetRelativeTransform (Variables|Default|GetShape)))) (.y (.scale (Transformation|GetRelativeTransform (Variables|Default|GetShape)))) (.z (.scale (Transformation|GetRelativeTransform (Variables|Default|GetShape))))))))
      (bind _output_get_2 (Variables|Default|SetShape _returnvalue))
      (Components|StaticMesh|SetStaticMesh _output_get_2 (Utilities|Array|Get(acopy) (Variables|Default|GetNew%20Mesh) (Variables|Default|GetType))))))

(event EventBeginPlay
  (Variables|Default|SetShape (Variables|Default|GetStaticMesh))
  (CallFunction|CEBEGIN))

(fn ConstructionScript)